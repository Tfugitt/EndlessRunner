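; Blueprint function library for an endless runner that manages the UI_EndlessRunner HUD widget.
; InitUI creates the widget for player 0, adds it to the viewport, resets the coin and speed texts and hides the game-over text.
; UpdateScore and GameOver find the live widget with GetAllWidgetsOfClass rather than a stored reference, then refresh both counters or reveal the game-over text.
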(fn UpdateScore
  (params (Score :type Score%20Structure))
  (bind _foundwidgets (Widget|GetAllWidgetsOfClass (LocalVariables|Get__WorldContext) "/Game/Libraries/UI_EndlessRunner.UI_EndlessRunner_C"))
  (Utilities|IsValid (Utilities|Array|Get(acopy) _foundwidgets)
    (:Is%20Valid
      (Rendering|Components|TextRender|SetText (Variables|/Game/Libraries/UI_EndlessRunner.UI_EndlessRunner_C|Gettxt_coins (Utilities|Array|Get(acopy) _foundwidgets)) (Utilities|Text|FormatText "Coins: {coins}" (.coins Score)))
      (Rendering|Components|TextRender|SetText (Variables|/Game/Libraries/UI_EndlessRunner.UI_EndlessRunner_C|Gettxt_Speed (Utilities|Array|Get(acopy) _foundwidgets)) (Utilities|Text|FormatText "Speed: {speed}" (.speed Score))))))

(fn InitUI
  (bind _returnvalue (UserInterface|CreateWidget "/Game/Libraries/UI_EndlessRunner.UI_EndlessRunner_C" (Game|GetPlayerController (LocalVariables|Get__WorldContext))))
  (UserInterface|Viewport|AddtoViewport _returnvalue 0)
  (Rendering|Components|TextRender|SetText (Variables|/Game/Libraries/UI_EndlessRunner.UI_EndlessRunner_C|Gettxt_coins _returnvalue) "Coins: 0")
  (Rendering|Components|TextRender|SetText (Variables|/Game/Libraries/UI_EndlessRunner.UI_EndlessRunner_C|Gettxt_Speed _returnvalue) "Speed: 0")
  (Widget|SetVisibility (Variables|/Game/Libraries/UI_EndlessRunner.UI_EndlessRunner_C|Gettxt_gameover _returnvalue) "Hidden"))

(fn GameOver
  (bind _foundwidgets (Widget|GetAllWidgetsOfClass (LocalVariables|Get__WorldContext) "/Game/Libraries/UI_EndlessRunner.UI_EndlessRunner_C"))
  (Utilities|IsValid (Utilities|Array|Get(acopy) _foundwidgets)
    (:Is%20Valid
      (Widget|SetVisibility (Variables|/Game/Libraries/UI_EndlessRunner.UI_EndlessRunner_C|Gettxt_gameover (Utilities|Array|Get(acopy) _foundwidgets)) "Visible"))))