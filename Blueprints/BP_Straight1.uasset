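; BP_Straight1 is an actor that lays out a row of coin pickups along its spline when play begins.
; SpawnCoinsOnSpline spawns fifteen BP_Coin actors, placing each at the world location for spline time equal to its loop index, with the player pawn as instigator.
; Each coin's yaw increases with its index, staggering the rotations across roughly a half turn.
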(event EventBeginPlay
  (CallFunction|SpawnCoinsonSpline (Variables|Default|GetSpline)))

(event Collision|EventActorBeginOverlap
  (params (OtherActor :type Actor%20Object%20Reference)))

(event EventTick
  (params (DeltaSeconds :type Float%20%28single-precision%29)))

(fn ConstructionScript)

(fn SpawnCoinsonSpline
  (params (Spline :type Spline%20Component%20Object%20Reference))
  (for _index (range 0 14)
    (Game|SpawnActorfromClass "/Game/Blueprints/BP_Coin.BP_Coin_C" (Math|Transform|MakeTransform (Spline|GetLocationatTime Spline (Math|Conversions|ToFloat(Integer) _index) "World" false) (Math|Rotator|MakeRotator 0.0 0.0 (* (/ (Math|Conversions|ToFloat(Integer) _index) 15.0) 1.8e+02))) "Undefined" "MultiplyWithRoot" 0 (Game|Player|GetPlayerPawn 0))))