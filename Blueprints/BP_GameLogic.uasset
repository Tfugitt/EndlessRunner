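; Game logic Blueprint for an endless runner: it builds the track, tracks coins and score, and ends the run on a crash.
; On BeginPlay it spawns segments from TrackPlacement, caches placed coins and binds to BP_Bot's hit event.
; Coin hits disable the coin and update score, while box component hits stop the bot and trigger GameOver.
; Tick fakes endless track by teleporting the player back past an X threshold and re-enabling coins.
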(event Custom|WallHitter
  (params (OtherActor :type Actor%20Object%20Reference) (OtherComponent :type Actor%20Component%20Object%20Reference))
  (CallFunction|WallDetectorEvent OtherActor OtherComponent))

(event EventBeginPlay
  (CallFunction|TrackSpawner)
  (CallFunction|CoinPopulation)
  (CallFunction|WallDetector (delegate Custom|WallHitter))
  (CallFunction|InitUI))

(event EventTick
  (params (DeltaSeconds :type Float%20%28single-precision%29))
  (CallFunction|LevelLoop))

(fn ConstructionScript)

(fn TrackSpawner
  (for (_array_element _array_index) (LocalVariables|GetTrackPlacement)
    (switch int _array_element
      (:0
        (Game|SpawnActorfromClass "/Game/Blueprints/BP_Straight1.BP_Straight1_C" (Math|Transform|MakeTransform (Math|Vector|MakeVector (Math|Conversions|ToFloat(Integer) (* _array_index 2000)) 0.0 0.0) "0, 0, 0" "1.000000,1.000000,1.000000") "Undefined" "MultiplyWithRoot" 0 0))
      (:1
        (Game|SpawnActorfromClass "/Game/Blueprints/BP_Straight.BP_Straight_C" (Math|Transform|MakeTransform (Math|Vector|MakeVector (Math|Conversions|ToFloat(Integer) (* _array_index 2000)) 0.0 0.0) "0, 0, 0" "1.000000,1.000000,1.000000") "Undefined" "MultiplyWithRoot" 0 0))
      (:2
        (Game|SpawnActorfromClass "/Game/Blueprints/BP_Straight2.BP_Straight2_C" (Math|Transform|MakeTransform (Math|Vector|MakeVector (Math|Conversions|ToFloat(Integer) (* _array_index 2000)) 0.0 0.0) "0, 0, 0" "1.000000,1.000000,1.000000") "Undefined" "MultiplyWithRoot" 0 0)))))

(fn CoinPopulation
  (bind _outactors (Actor|GetAllActorsOfClass "/Game/Blueprints/BP_Coin.BP_Coin_C"))
  (Variables|Default|SetCoinPlacement _outactors))

(fn WallDetector
  (params (Event :type Delegate%20%28by%20ref%29))
  (bind _asbp_bot (Utilities|Casting|CastToBP_Bot (Game|Player|GetPlayerPawn 0)))
  (EventDispatchers|BindEventtoBotHitSomething _asbp_bot Event))

(fn WallStopper
  (bind _asbp_bot (Utilities|Casting|CastToBP_Bot (Game|Player|GetPlayerPawn 0)))
  (Variables|/Game/Assets/Blueprints/Character/BP_Bot.BP_Bot_C|SetIsRunning _asbp_bot false))

(fn CoinReset
  (for _array_element (Variables|Default|GetCoinPlacement)
    (Default|Enable _array_element true)))

(fn LevelLoop
  (bind _returnvalue (Game|Player|GetPlayerPawn 0))
  (bind _output_get (Variables|Default|SetVector (Transformation|GetActorLocation _returnvalue)))
  (bind _output_get_2 (Variables|Default|SetRotator (Transformation|GetActorRotation _returnvalue)))
  (if (> (.X (Class|KismetMathLibrary|BreakVector3f _output_get)) 5e+03)
    (Transformation|Teleport _returnvalue (Math|Vector|MakeVector 2e+03 (.Y (Class|KismetMathLibrary|BreakVector3f _output_get)) (.Z (Class|KismetMathLibrary|BreakVector3f _output_get))) _output_get_2)
    (CallFunction|CoinReset)))

(fn WallDetectorEvent
  (params (HitBot :type Actor%20Object%20Reference) (HitDetected :type Actor%20Component%20Object%20Reference))
  (bind _asbp_coin (Utilities|Casting|CastToBP_Coin HitBot)
    (:then
      (Default|Enable _asbp_coin false)
      (bind _asbp_bot (Utilities|Casting|CastToBP_Bot (Game|Player|GetPlayerPawn 0)))
      (bind _result (Math|Integer|IncrementInt (Variables|Default|GetCoinTotal))
        (:%20%20
          (CallFunction|UpdateScore (Utilities|Struct|MakeScore _result (Variables|/Script/Engine.CharacterMovementComponent|GetMaxWalkSpeed (Variables|/Script/Engine.Character|GetCharacterMovement _asbp_bot)))))))
    (:CastFailed
      (Utilities|Casting|CastToBoxComponent HitDetected)
      (CallFunction|WallStopper)
      (CallFunction|GameOver))))