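; BP_Ramp is a level ramp that tilts up and down in response to one or more designer-assigned trigger actors.
; It binds to each trigger's BP_InteractionComponent and counts activations, raising once the required number is reached, as in BP_Door.
; Any deactivation decrements the count and lowers the ramp.
; The RiseRamp timeline plays or reverses, scaling a designer-set angle to drive the mesh's relative pitch.
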(event Custom|OnInteract
  (params (On :type Boolean))
  ;[0.3892 1 0.8243] Like the door and other game objects, the ramp can reqyire more than one trigger. You can specify an array of triggers and how many are required to be active, which makes it quite flexible. For more details check out the BP_Door.
  (if On
    (bind _result (Math|Integer|IncrementInt (Variables|Default|GetTriggersActive))
      (:%20%20
        (if (>= _result (Variables|Default|GetTriggersNeeded))
          (CallFunction|ToUpperLocation))))
    (else
      (Variables|Default|SetTriggersActive (Math|Integer|Max(Integer) (- (Variables|Default|GetTriggersActive) 1)))
      (CallFunction|ToLowerLocation))))

(event Custom|ToUpperLocation
  ;[0.4469 0.6458 1] Using a timeline and an angle specified by the level designer to rotate the ramp up or down.
  (bind _riseramp (Timeline|RiseRamp Play)
    (:Update
      (Transformation|SetRelativeRotation (Variables|Default|GetRampMesh) (Math|Rotator|MakeRotator 0.0 (* _riseramp (Variables|Default|GetUpperAngle)) 0.0) false false))))

(event Custom|ToLowerLocation
  ;[0.4469 0.6458 1] Using a timeline and an angle specified by the level designer to rotate the ramp up or down.
  (bind _riseramp (Timeline|RiseRamp Reverse)
    (:Update
      (Transformation|SetRelativeRotation (Variables|Default|GetRampMesh) (Math|Rotator|MakeRotator 0.0 (* _riseramp (Variables|Default|GetUpperAngle)) 0.0) false false))))

(event EventBeginPlay
  ;[0.3892 1 0.8243] Like the door and other game objects, the ramp can reqyire more than one trigger. You can specify an array of triggers and how many are required to be active, which makes it quite flexible. For more details check out the BP_Door.
  (if (> (Utilities|Array|Length (Variables|Default|GetTriggers)) 0)
    (for _array_element (Variables|Default|GetTriggers)
      (EventDispatchers|AssignOnInteract (Actor|GetComponentbyClass _array_element "/Game/Assets/Blueprints/Abilities/BP_InteractionComponent.BP_InteractionComponent_C") (delegate Custom|OnInteract)))))

(fn ConstructionScript)